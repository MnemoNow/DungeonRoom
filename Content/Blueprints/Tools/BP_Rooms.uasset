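; BP_Rooms is a construction-script tool that builds a simple modular room shell from plane meshes.
; Nested loops tile the floor on a 100-unit grid sized by X and Y counts, with each outer step also adding a plane that overlaps its row's first tile.
; A final loop stacks rotated, offset planes into a single wall column of configurable height.
; The event graph has no active logic.
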(fn `UserConstructionScript`
  ;[1 0.2837 0.204 0.5] Need make a floor first... Floor X vector
  (for _index (range (`self.X - FloorVector(M)`))
    (bind _returnvalue (* _index 100))
    (bind _returnvalue_2 (`AddComponent|NODE_AddStaticMeshComponent-1` :`RelativeTransform` (`KismetMathLibrary.MakeTransform` (`KismetMathLibrary.MakeVector` _returnvalue))))
    (bind _output_get (set `self.X FloorProp` _returnvalue_2))
    (`StaticMeshComponent.SetStaticMesh` _output_get "/Game/OBJ/UsefullPlane.UsefullPlane")
    ; Floor Y
    (for _index_2 (range (`self.Y - FloorVector(M)`))
      (bind _returnvalue_3 (`AddComponent|NODE_AddStaticMeshComponent-2` :`RelativeTransform` (`KismetMathLibrary.MakeTransform` (`KismetMathLibrary.MakeVector` _returnvalue (* _index_2 100)))))
      (`StaticMeshComponent.SetStaticMesh` _returnvalue_3 "/Game/OBJ/UsefullPlane.UsefullPlane")))
  ; First walls - Height
  (for _index_3 (range (`self.Wall 1 - Height`))
    (bind _returnvalue_4 (`AddComponent|NODE_AddStaticMeshComponent-3` :`RelativeTransform` (`KismetMathLibrary.MakeTransform` (`KismetMathLibrary.MakeVector` 0.0 0.0 (* _index_3 100.0)) (struct :`Roll` 90.0))))
    (bind _output_get_2 (set `self.WallProp` _returnvalue_4))
    (`StaticMeshComponent.SetStaticMesh` _output_get_2 "/Game/OBJ/UsefullPlane.UsefullPlane")
    (`SceneComponent.K2_AddLocalOffset` (`self.WallProp`) (0.0 -50.0 -50.0) false false)))